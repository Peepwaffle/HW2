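; BP_Target is a shootable target that counts toward the player's goal when destroyed.
; Each hit from a BP_FirstPersonProjectile removes a fixed amount of Health, and other collisions are ignored.
; When Health equals exactly zero, it increments TargetsHit on the player's BP_FirstPersonCharacter, calls CheckGoal there, and destroys itself.
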(event Collision|EventHit
  (params (MyComp :type Primitive%20Component%20Object%20Reference) (Other :type Actor%20Object%20Reference) (OtherComp :type Primitive%20Component%20Object%20Reference) (bSelfMoved :type Boolean) (HitLocation :type Vector :default "0, 0, 0") (HitNormal :type Vector :default "0, 0, 0") (NormalImpulse :type Vector :default "0, 0, 0") (Hit :type Hit%20Result%20Structure%20%28by%20ref%29))
  (Utilities|Casting|CastToBP_FirstPersonProjectile Other)
  (bind _output_get (Variables|Default|SetHealth (- (Variables|Default|GetHealth) 20)))
  (if (== _output_get 0)
    (bind _asbp_first_person_character_2 (Utilities|Casting|CastToBP_FirstPersonCharacter2 (Game|GetPlayerCharacter 0)))
    (Variables|/Game/FirstPerson/Blueprints/BP_FirstPersonCharacter2.BP_FirstPersonCharacter2_C|SetTargets%20Hit _asbp_first_person_character_2 (+ (Variables|/Game/FirstPerson/Blueprints/BP_FirstPersonCharacter2.BP_FirstPersonCharacter2_C|GetTargets%20Hit _asbp_first_person_character_2) 1))
    (Default|CheckGoal _asbp_first_person_character_2)
    (Actor|DestroyActor)))

(fn ConstructionScript)